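; MLSUDPReceiver is an actor that receives simulation data over UDP and passes it to an MLS implementation object.
; BeginPlay opens a local UDP socket and stores whether it is ready.
; Each Tick polls for new packets and forwards four floats (current height, lateral X and Y movement, external setpoint) through DeliverDataMessage on MLSImplRef.
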(event `self.ReceiveBeginPlay`
  (bind _returnvalue (`self.StartUDPReceiver` "sock1" "127.0.0.1" 9988))
  (set `self.RcvSocketReady` _returnvalue))

(event `self.ReceiveTick`
  (params (DeltaSeconds :type "Float (single-precision)"))
  (if (`self.RcvSocketReady`)
    (bind _returnvalue (`self.IsNewDataReady`))
    (if _returnvalue
      (bind _returnvalue_2 (`self.GetData`))
      (bind (_float1 _float2 _float3 _float4) (break `UDPData` _returnvalue_2))
      (message `/Game/Blueprints/MLSDDeliverInterface.DeliverData` (`self.MLSImplRef`) _float1 _float2 _float3 _float4))))

(fn `UserConstructionScript`)