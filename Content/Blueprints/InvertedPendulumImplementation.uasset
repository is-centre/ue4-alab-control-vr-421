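; Actor Blueprint that visualizes an inverted pendulum by driving linked caret and left and right pendulum actors.
; On BeginPlay it caches the caret's starting location and the left pendulum's starting rotation.
; The DeliverData event applies a received position and angle as offsets from those baselines, moving the caret along negated world X and pitching both pendulums after converting radians to degrees.
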(event `self.ReceiveBeginPlay`
  (set `self.OriginalCaretLocation` (`self.K2_GetActorLocation` (`self.LinkCaret`)))
  (set `self.OriginalPendulumRotation` (`self.K2_GetActorRotation` (`self.LinkPendulumLeft`))))

(event `/Game/Blueprints/InvpDDeliverInterface.DeliverData`
  (params (CaretPosition :type "Float (single-precision)") (PendulumAngle :type "Float (single-precision)"))
  (bind _returnvalue (`KismetMathLibrary.MakeRotator` (.roll (`self.OriginalPendulumRotation`)) (+ (.pitch (`self.OriginalPendulumRotation`)) (`KismetMathLibrary.RadiansToDegrees` PendulumAngle)) (.yaw (`self.OriginalPendulumRotation`))))
  (`self.K2_SetActorLocation` (`self.LinkCaret`) (`KismetMathLibrary.MakeVector` (+ (.x (`self.OriginalCaretLocation`)) (* CaretPosition -1.0)) (.y (`self.OriginalCaretLocation`)) (.z (`self.OriginalCaretLocation`))) false false)
  (`self.K2_SetActorRotation` (`self.LinkPendulumLeft`) _returnvalue false)
  (`self.K2_SetActorRotation` (`self.LinkPendulumRight`) _returnvalue false))

(fn `UserConstructionScript`)