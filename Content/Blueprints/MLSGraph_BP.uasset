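; MLSGraph_BP is an actor that feeds height readings to a time plot in its MLSGraph widget, comparing a sphere's actual and desired height.
; AddActualHeight and AddDesiredHeight each cast the Widget component's user widget to MLSGraph and append the value to PlotPosition under the SphereActual or SphereSP series.
; Data arrives only through calls to these functions, as the event graph and construction script are empty.
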(event `self.ReceiveBeginPlay`)

(fn `AddActualHeight`
  (params (DataPoint :type "Float (double-precision)"))
  (bind _asmlsgraph (cast `/Game/Blueprints/MLSGraph` (`WidgetComponent.GetUserWidgetObject` (`self.Widget`))))
  (`SimpleTimeSeriesPlot.BP_AddDatapointNow` (`/Game/Blueprints/MLSGraph.PlotPosition` _asmlsgraph) "SphereActual" DataPoint))

(fn `AddDesiredHeight`
  (params (DataPoint :type "Float (double-precision)"))
  (bind _asmlsgraph (cast `/Game/Blueprints/MLSGraph` (`WidgetComponent.GetUserWidgetObject` (`self.Widget`))))
  (`SimpleTimeSeriesPlot.BP_AddDatapointNow` (`/Game/Blueprints/MLSGraph.PlotPosition` _asmlsgraph) "SphereSP" DataPoint))

(fn `UserConstructionScript`)