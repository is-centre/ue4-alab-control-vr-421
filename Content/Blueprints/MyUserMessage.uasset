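; MyUserMessage is an actor that displays a text message to the user through a UserMessages widget held in its WidgetUserMsg component.
; UpdateText sets the message string and ChangeTextOpacity sets its opacity, both by casting the component's widget to UserMessages and editing TxtUserMessage.
; ShowText toggles the visibility of the widget component without propagating to children.
; The event graph and construction script are empty, so other code drives it through these functions.
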(event `self.ReceiveBeginPlay`)

(event `self.ReceiveTick`
  (params (DeltaSeconds :type "Float (single-precision)")))

(fn `ChangeTextOpacity`
  (params (Opacity :type "Float (double-precision)"))
  (bind _asuser_messages (cast `/Game/Blueprints/UserMessages` (`WidgetComponent.GetUserWidgetObject` (`self.Widget_UserMsg`))))
  (`TextBlock.SetOpacity` (`/Game/Blueprints/UserMessages.txtUserMessage` _asuser_messages) Opacity))

(fn `ShowText`
  (params (Visibility :type Boolean))
  (`SceneComponent.SetVisibility` (`self.Widget_UserMsg`) Visibility false))

(fn `UpdateText`
  (params (UserMessageTxt :type String))
  (bind _asuser_messages (cast `/Game/Blueprints/UserMessages` (`WidgetComponent.GetUserWidgetObject` (`self.Widget_UserMsg`))))
  (`TextBlock.SetText` (`/Game/Blueprints/UserMessages.txtUserMessage` _asuser_messages) (`KismetTextLibrary.Conv_StringToText` UserMessageTxt)))

(fn `UserConstructionScript`)