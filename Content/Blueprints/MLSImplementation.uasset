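; Magnetic levitation system actor that visualizes a ball's position relative to a magnet from delivered simulation data.
; DeliverData scales lateral movement into relative X/Y and maps height, normalized by the maximum magnet distance, to an inverted Z, so larger values sit lower.
; It also stores the height and external SP value.
; Ball begin and end overlaps are re-broadcast through event dispatchers with the other actor.
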(event `/Game/Blueprints/MLSDDeliverInterface.DeliverData`
  (params (CurrentHeight :type "Float (single-precision)") (LateralMovementX :type "Float (single-precision)") (LateralMovementY :type "Float (single-precision)") (ExternalSP :type "Float (single-precision)"))
  (`SceneComponent.K2_SetRelativeLocation` (`self.mls-ball-only_optimized`) (`KismetMathLibrary.MakeVector` (* LateralMovementX 2.5) (* LateralMovementY 2.5) (- 2.0 (* 2.0 (/ CurrentHeight (`self.MaxDistFromMagnet`))))) false false)
  (set `self.TheHeight` CurrentHeight)
  (set `self.TheExternalSP` ExternalSP))

(event `self.mls-ball-only_optimized.OnComponentBeginOverlap`
  (params (OverlappedComponent :type "PrimitiveComponent Object Reference") (OtherActor :type "Actor Object Reference") (OtherComp :type "PrimitiveComponent Object Reference") (OtherBodyIndex :type Integer) (bFromSweep :type Boolean) (SweepResult :type "HitResult Structure (by ref)"))
  (`self.BallBeginOverlapping` OtherActor))

(event `self.mls-ball-only_optimized.OnComponentEndOverlap`
  (params (OverlappedComponent :type "PrimitiveComponent Object Reference") (OtherActor :type "Actor Object Reference") (OtherComp :type "PrimitiveComponent Object Reference") (OtherBodyIndex :type Integer))
  (`self.BallEndOverlapping` OtherActor))

(event `self.ReceiveTick`
  (params (DeltaSeconds :type "Float (single-precision)")))

(fn `UserConstructionScript`)